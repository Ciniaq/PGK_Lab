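; Paper2D eagle enemy that patrols horizontally and kills the player on contact while alive.
; Tick moves the capsule a fixed step per frame between its spawn point and an X offset, flipping the sprite at each end.
; Overlapping the KillBox stops the eagle, increments the player's kill count, bounces them upward, then plays a death flipbook before destroying the actor.
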(event `self.ReceiveBeginPlay`
  (bind _output_get (set `self.StartingLocation` (`SceneComponent.K2_GetComponentLocation` (`self.CapsuleComponent`))))
  (set `self.MaxLocation` (+ _output_get (`KismetMathLibrary.MakeVector` (`self.xLocation`)))))

(event `self.ReceiveActorBeginOverlap`
  (params (OtherActor :type "Actor Object Reference"))
  (bind _returnvalue (`GameplayStatics.GetPlayerCharacter` 0))
  (if (== OtherActor _returnvalue)
    (if (`self.isAlive`)
      (`KismetSystemLibrary.PrintString` "eagle")
      (bind _asbp_paper_character (cast `/Game/Character/BP_PaperCharacter` _returnvalue))
      (`/Game/Character/BP_PaperCharacter.Kill Player` _asbp_paper_character))))

(event `self.ReceiveTick`
  (params (DeltaSeconds :type "Float (single-precision)"))
  (bind _returnvalue_x (`KismetMathLibrary.BreakVector` (`SceneComponent.K2_GetComponentLocation` (`self.CapsuleComponent`))))
  (bind _returnvalue_x_2 (`KismetMathLibrary.BreakVector` (`SceneComponent.K2_GetComponentLocation` (`self.CapsuleComponent`))))
  (if (`self.CanMove`)
    (if (`self.bIsMovingRight`)
      (if (> _returnvalue_x (`KismetMathLibrary.BreakVector3f` (`self.MaxLocation`)))
        (set `self.bIsMovingRight` false)
        (`SceneComponent.K2_AddRelativeRotation` (`self.Sprite`) (struct :`Yaw` 180.0) false false :!label _label)
        (else
          (`SceneComponent.K2_SetWorldLocation` (`self.CapsuleComponent`) (+ (`SceneComponent.K2_GetComponentLocation` (`self.CapsuleComponent`)) (0.5 0.0 0.0)) false false)))
      (elif (< _returnvalue_x_2 (`KismetMathLibrary.BreakVector3f` (`self.StartingLocation`)))
        (set `self.bIsMovingRight` true)
        (goto _label)
        (else
          (`SceneComponent.K2_SetWorldLocation` (`self.CapsuleComponent`) (+ (`SceneComponent.K2_GetComponentLocation` (`self.CapsuleComponent`)) (-0.5 0.0 0.0)) false false))))))

(event `self.KillBox.OnComponentBeginOverlap`
  (params (OverlappedComponent :type "PrimitiveComponent Object Reference") (OtherActor :type "Actor Object Reference") (OtherComp :type "PrimitiveComponent Object Reference") (OtherBodyIndex :type Integer) (bFromSweep :type Boolean) (SweepResult :type "HitResult Structure (by ref)"))
  (if (and (== OtherActor (`GameplayStatics.GetPlayerCharacter` 0)) (`self.isAlive`))
    (set `self.isAlive` false)
    (set `self.CanMove` false)
    (`PaperFlipbookComponent.SetFlipbook` (`self.Sprite`) "/Game/assets/PNG/sprites/enemy-death/FB_Death.FB_Death")
    (bind _asbp_paper_character (cast `/Game/Character/BP_PaperCharacter` (`GameplayStatics.GetPlayerCharacter` 0)))
    (set `/Game/Character/BP_PaperCharacter.KilledEnemies` (+ (`/Game/Character/BP_PaperCharacter.KilledEnemies` _asbp_paper_character) 1) _asbp_paper_character)
    (bind _charactermovement (`Character.CharacterMovement` _asbp_paper_character))
    (set `MovementComponent.Velocity` (0.0 0.0 0.0) _charactermovement)
    (`CharacterMovementComponent.AddImpulse` _charactermovement (0.0 0.0 250.0) true)
    (`KismetSystemLibrary.PrintText` "killed")
    (`KismetSystemLibrary.Delay` (`PaperFlipbookComponent.GetFlipbookLength` (`self.Sprite`)))
    (`self.K2_DestroyActor`)))

(fn `UserConstructionScript`)