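; BP_FinishTree is the level's finish point, gated on the player having collected at least three keys.
; On BeginPlay it caches the player's BP_PaperCharacter, then checks that character's Keys count when it enters the Box trigger.
; Too few keys shows the HUD's MoreKeysText until the player leaves the box, while enough keys adds the WBP_EndLevel widget to the viewport.
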(event `self.ReceiveBeginPlay`
  (bind _asbp_paper_character (cast `/Game/Character/BP_PaperCharacter` (`GameplayStatics.GetPlayerCharacter` 0)))
  (set `self.As BP Paper Character` _asbp_paper_character))

(event `self.Box.OnComponentBeginOverlap`
  (params (OverlappedComponent :type "PrimitiveComponent Object Reference") (OtherActor :type "Actor Object Reference") (OtherComp :type "PrimitiveComponent Object Reference") (OtherBodyIndex :type Integer) (bFromSweep :type Boolean) (SweepResult :type "HitResult Structure (by ref)"))
  (bind _as_bp_paper_character (`self.As BP Paper Character`))
  (if (== OtherActor _as_bp_paper_character)
    (if (< (`/Game/Character/BP_PaperCharacter.Keys` _as_bp_paper_character) 3)
      (`KismetSystemLibrary.PrintString` "Finish point overlapping")
      (bind _ashud_class (cast `/Game/Character/HudClass` (`PlayerController.GetHUD` (`GameplayStatics.GetPlayerController` 0))))
      (`Widget.SetVisibility` (`/Game/WBP_HUD.moreKeysText` (`/Game/Character/HudClass.MyHud` _ashud_class)) "Visible")
      (else
        (`KismetSystemLibrary.PrintString` "level finished")
        (bind _returnvalue (`|CreateWidget` "/Game/WBP_EndLevel.WBP_EndLevel_C"))
        (`UserWidget.AddToViewport` _returnvalue 0)))))

(event `self.Box.OnComponentEndOverlap`
  (params (OverlappedComponent :type "PrimitiveComponent Object Reference") (OtherActor :type "Actor Object Reference") (OtherComp :type "PrimitiveComponent Object Reference") (OtherBodyIndex :type Integer))
  (if (== OtherActor (`self.As BP Paper Character`))
    (bind _ashud_class (cast `/Game/Character/HudClass` (`PlayerController.GetHUD` (`GameplayStatics.GetPlayerController` 0))))
    (`Widget.SetVisibility` (`/Game/WBP_HUD.moreKeysText` (`/Game/Character/HudClass.MyHud` _ashud_class)) "Hidden")))

(fn `UserConstructionScript`)