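; Player Paper2D character for a side-scrolling game that moves along X, jumps, and collects nuts, keys and hearts.
; Tick swaps idle, run and jump flipbooks from movement state and flips control rotation to face the travel direction.
; KillPlayer removes a heart, teleports to the position saved at BeginPlay, and opens the death widget when none remain.
; BeginPlay also starts a looping timer, apparently for the Timer counter.
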(event `self.ReceiveBeginPlay`
  (`KismetSystemLibrary.K2_SetTimerDelegate` (`|CreateDelegate` :!event `TimerFun`) 1.0 true)
  (set `self.Spawn Transform` (.location (`self.GetTransform`))))

(event `self.ReceiveTick`
  (params (DeltaSeconds :type "Float (single-precision)"))
  (`self.UpdateAnimation`)
  (`self.UpdateCustomRotation`))

(event `Kill Player`
  (bind _returnvalue (`GameplayStatics.GetPlayerController` 0))
  (bind _output_get (set `self.Hearts` (- (`self.Hearts`) 1)))
  (`KismetSystemLibrary.PrintText` (`|FormatText` "Hearts left: {left}" _output_get))
  (`self.K2_SetActorLocation` (`self.Spawn Transform`) false true)
  (if (not (> _output_get 0))
    (bind _returnvalue_2 (`|CreateWidget` "/Game/WBP_Death.WBP_Death_C"))
    (`UserWidget.AddToViewport` _returnvalue_2 0)
    (`WidgetBlueprintLibrary.SetInputMode_GameAndUIEx` _returnvalue _returnvalue_2)
    (set `PlayerController.bShowMouseCursor` true _returnvalue)))

(event `InputAxis|MoveRight`
  (params (AxisValue :type "Float (single-precision)"))
  (`self.AddMovementInput` (1.0 0.0 0.0) AxisValue))

(event `InputAction|InputJump`
  (params (Key :type "Key Structure"))
  (:`Pressed`
    (`self.Jump`))
  (:`Released`
    (`self.StopJumping`)))

(event `UpdateAnimation`
  (`PaperFlipbookComponent.SetFlipbook` (`self.Sprite`) (select `bool` (`NavMovementComponent.IsFalling` (`self.CharacterMovement`)) :`false` (select `bool` (> (`KismetMathLibrary.VSize` (`MovementComponent.Velocity` (`self.CharacterMovement`))) 0.0) :`false` "/Game/assets/PNG/sprites/player/idle/player-idle.player-idle" :`true` "/Game/assets/PNG/sprites/player/run/player-run.player-run" :!type "PaperFlipbook Object Reference") :`true` "/Game/assets/PNG/sprites/player/jump/player-jump.player-jump")))

(event `UpdateCustomRotation`
  (`/Engine/EditorBlueprintResources/StandardMacros.CompareFloat` (`KismetMathLibrary.BreakVector3f` (`MovementComponent.Velocity` (`self.CharacterMovement`)))
    (:`>`
      (`Controller.SetControlRotation` (`self.GetController`) (`KismetMathLibrary.MakeRotator` 0.0)))
    (:`<`
      (`Controller.SetControlRotation` (`self.GetController`) (`KismetMathLibrary.MakeRotator` 0.0 0.0 180.0)))))

(fn `AddHeart`
  (params (quantity :type Integer))
  (set `self.Hearts` (+ (`self.Hearts`) quantity))
  (`KismetSystemLibrary.PrintText` (`|FormatText` "Added {num} heart" quantity) true true (struct :`R` 0.051729 :`G` 1.0 :`A` 1.0) 5.0))

(fn `AddKey`
  (params (quantity :type Integer))
  (set `self.Keys` (+ (`self.Keys`) quantity))
  (`KismetSystemLibrary.PrintText` (`|FormatText` "Added {num} keys" quantity) true true (struct :`R` 1.0 :`G` 0.366855 :`A` 1.0) 5.0))

(fn `AddNut`
  (params (quantity :type Integer))
  (set `self.Nuts` (+ (`self.Nuts`) quantity))
  (`KismetSystemLibrary.PrintText` (`|FormatText` "Added {num} nut" quantity) true true (struct :`R` 1.0 :`G` 0.059606 :`A` 1.0) 5.0))

(fn `TimerFun`
  (`/Engine/EditorBlueprintResources/StandardMacros.IncrementInt` (`self.Timer`)))

(fn `UserConstructionScript`)